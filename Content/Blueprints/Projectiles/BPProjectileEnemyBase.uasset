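; Base enemy projectile that flies along its local axes and damages the player on impact.
; Tick moves it by Speed times delta time using a swept local offset.
; A mesh hit applies Damage only when the other actor is BPPlayer, then destroys the projectile whatever it struck.
; The construction script sets the actor's scale from the Scale variable.
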(event OnComponentHit(ProjectileMesh)
  (params (HitComponent :type Primitive%20Component%20Object%20Reference) (OtherActor :type Actor%20Object%20Reference) (OtherComp :type Primitive%20Component%20Object%20Reference) (NormalImpulse :type Vector :default "0, 0, 0") (Hit :type Hit%20Result%20Structure%20%28by%20ref%29))
  ;[1 1 1] Collision Events
  (bind _asbpplayer (Utilities|Casting|CastToBPPlayer OtherActor)
    (:then
      (Game|Damage|ApplyDamage _asbpplayer (Variables|Default|GetDamage) 0 0))
    (:CastFailed
      _))
  (Actor|DestroyActor))

(event EventTick
  (params (DeltaSeconds :type Float%20%28single-precision%29))
  ;[1 1 1] Move Projectile
  (Transformation|AddActorLocalOffset (* (Variables|Default|GetSpeed) DeltaSeconds) true false))

(fn ConstructionScript
  (Transformation|SetActorScale3D (Variables|Default|GetScale)))