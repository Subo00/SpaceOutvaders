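; BPLaserEnemy is a short-lived enemy laser shot that hits instantly via line trace rather than traveling.
; On BeginPlay it traces from its Cube forward for a fixed range and stretches a particle beam between the Cube and the hit location.
; If the trace hits a BPPlayer it applies Damage, then the actor destroys itself after a brief delay.
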(event EventBeginPlay
  (bind _cube (Variables|Default|GetCube))
  (bind _returnvalue (Transformation|GetWorldLocation _cube))
  (Class|ParticleSystemComponent|SetBeamSourcePoint (Variables|Default|GetParticleSystem) 0 (Transformation|GetWorldLocation (Variables|Default|GetCube)))
  (bind _outhit (Collision|LineTraceForObjects _returnvalue (+ _returnvalue (* (Math|Vector|GetForwardVector _cube) 5e+03)) (Variables|Default|GetObjectTypes) false 0 "None"))
  (bind _output_get (Variables|Default|SetEndLocation (.Location (Collision|BreakHitResult _outhit))))
  (Class|ParticleSystemComponent|SetBeamTargetPoint (Variables|Default|GetParticleSystem) 0 _output_get)
  (bind _asbpplayer (Utilities|Casting|CastToBPPlayer (.HitActor (Collision|BreakHitResult _outhit)))
    (:then
      (Game|Damage|ApplyDamage _asbpplayer (Variables|Default|GetDamage) 0 0))
    (:CastFailed
      _))
  (Utilities|FlowControl|Delay 0.1)
  (Actor|DestroyActor))

(event Collision|EventActorBeginOverlap
  (params (OtherActor :type Actor%20Object%20Reference)))

(event EventTick
  (params (DeltaSeconds :type Float%20%28single-precision%29)))

(fn ConstructionScript)