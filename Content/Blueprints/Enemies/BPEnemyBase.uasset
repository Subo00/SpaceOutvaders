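; Base enemy for what appears to be a Space Invaders-style shooter, sweeping sideways at constant speed.
; Hitting a static mesh actor moves it down for a second, then reverses its direction.
; It explodes on hitting an island, destroying both, or the player, dealing damage.
; It registers with BPGameMode on spawn; only death by damage deregisters it, awards score and may spawn a random pickup.
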(event EventBeginPlay
  ;[1 1 1] Event Begin Play
  (bind _asbpgame_mode (Utilities|Casting|CastToBPGameMode (Game|GetGameMode)))
  (bind _output_get (Variables|Default|SetBPGameMode _asbpgame_mode))
  (Default|AddEnemy _output_get))

(event EventTick
  (params (DeltaSeconds :type Float%20%28single-precision%29))
  ;[1 1 1] Movement
  (if (Variables|Default|GetbMoveDown)
    (Transformation|SetActorLocation (+ (Transformation|GetActorLocation) (* (Math|Vector|RotateVector (Math|Vector|MakeVector 0.0 0.0 (* (Variables|Float|GetMoveSpeed) -1.0)) "0, 0, 0") DeltaSeconds)) true false)
    (else
      (Transformation|SetActorLocation (+ (Transformation|GetActorLocation) (* (Math|Vector|RotateVector (Math|Vector|MakeVector (* (Variables|Float|GetMoveSpeed) (Math|Float|SelectFloat -1.0 1.0 (Variables|Default|GetbMoveRight))) 0.0 0.0) "0, 0, 0") DeltaSeconds)) true false))))

(event Collision|EventHit
  (params (MyComp :type Primitive%20Component%20Object%20Reference) (Other :type Actor%20Object%20Reference) (OtherComp :type Primitive%20Component%20Object%20Reference) (bSelfMoved :type Boolean) (HitLocation :type Vector :default "0, 0, 0") (HitNormal :type Vector :default "0, 0, 0") (NormalImpulse :type Vector :default "0, 0, 0") (Hit :type Hit%20Result%20Structure%20%28by%20ref%29))
  ;[1 1 1] Enemy Hit Something
  (Utilities|Casting|CastToStaticMeshActor Other
    (:then
      (Variables|Default|SetbMoveDown true)
      (Utilities|FlowControl|Delay 1.0)
      (Variables|Default|SetbMoveDown false)
      (Variables|Default|SetbMoveRight (not (Variables|Default|GetbMoveRight))))
    (:CastFailed
      (bind _asbpisland (Utilities|Casting|CastToBPIsland Other)
        (:then
          (Audio|PlaySoundatLocation "/Game/Audio/Explosion.Explosion" "0, 0, 0" "0, 0, 0" 1.0 1.0 0.0 0 0 0)
          (Actor|DestroyActor)
          (Actor|DestroyActor _asbpisland))
        (:CastFailed
          (bind _asbpplayer (Utilities|Casting|CastToBPPlayer Other))
          (Game|Damage|ApplyDamage _asbpplayer 5e+01 0 0)
          (Audio|PlaySoundatLocation "/Game/Audio/Explosion.Explosion" "0, 0, 0" "0, 0, 0" 1.0 1.0 0.0 0 0 0)
          (Actor|DestroyActor))))))

(event Game|Damage|EventAnyDamage
  (params (Damage :type Float%20%28single-precision%29) (DamageType :type Damage%20Type%20Object%20Reference) (InstigatedBy :type Controller%20Object%20Reference) (DamageCauser :type Actor%20Object%20Reference))
  (bind _pickups (Variables|Default|GetPickUps))
  (bind _bpgamemode (Variables|Default|GetBPGameMode))
  ;[1 1 1] Enemy Death
  (Variables|Float|SetHealth (Math|Float|Clamp(Float) (- (Variables|Float|GetHealth) Damage) 0.0 (Variables|Float|GetMaxHealth)))
  (if (<= (Variables|Float|GetHealth) 0.0)
    (Default|RemoveEnemy _bpgamemode)
    (Default|AddScore _bpgamemode (Variables|Default|GetScore%20to%20Add))
    (if (<= (Math|Random|RandomFloatinRange 0.0 1.0) (Variables|Float|GetDropRate))
      (Game|SpawnActorfromClass (Utilities|Array|Get(acopy) _pickups (Math|Random|RandomIntegerinRange 0 (Utilities|Array|LastIndex _pickups))) (Transformation|GetActorTransform) "Undefined" 0 0))
    (Audio|PlaySoundatLocation "/Game/Audio/Explosion.Explosion" "0, 0, 0" "0, 0, 0" 1.0 1.0 0.0 0 0 0)
    (Actor|DestroyActor)))

(fn ConstructionScript
  (Variables|Float|SetHealth (Variables|Float|GetMaxHealth))
  (Transformation|SetRelativeRotation (Variables|Default|GetEnemyMesh) "0.000000,0.000000,-90.000000" false false))