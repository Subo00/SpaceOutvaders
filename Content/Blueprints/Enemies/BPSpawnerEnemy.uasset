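; Enemy wave spawner that starts a new, one-larger wave whenever the game mode's live enemy count reaches zero, checked on a looping timer.
; BeginWave splits the wave into rows stepped down in Z, alternating left-to-right and right-to-left helpers, plus a remainder row.
; The helpers spawn random classes at even X spacing; right-to-left spawns get MoveRight cleared.
; A boss row is supported, but its every-third-wave trigger is disconnected.
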(event Custom|WaveCheck
  (if (== (Variables|/Game/Blueprints/Misc/BPGameMode.BPGameMode_C|GetLiveEnemies (Variables|Default|GetBPGameMode)) 0)
    (CallFunction|BeginWave (Variables|Default|GetnumEnemies) (Variables|EnemyWave|GetWave1))
    (Variables|Default|SetnumEnemies (+ (Variables|Default|GetnumEnemies) 1))
    (Variables|Waves|SetWaveIndex (+ (Variables|Waves|GetWaveIndex) 1))))

(event EventBeginPlay
  ;[1 1 1] Event Begin Play
  (bind _asbpgame_mode (Utilities|Casting|CastToBPGameMode (Game|GetGameMode)))
  (Variables|Default|SetBPGameMode _asbpgame_mode)
  (bind _output_get (Variables|Float|SetLenghtMax (- (.x (Variables|Default|GetSpawnLocationLeft)) (.x (Variables|Default|GetSpawnLocationRight)))))
  (Variables|Float|SetStep (/ _output_get (Math|Conversions|ToFloat(Integer) (Variables|Default|GetMaxNumInRow))))
  (bind _returnvalue (Utilities|Time|SetTimerbyFunctionName 0 "WaveCheck" 1.0 true))
  (Variables|Default|SetWaveTimer _returnvalue))

(fn ConstructionScript)

(fn BeginWave
  (params (WaveTotal :type Integer) (WaveEnemies :type Array%20of%20BP%20Enemy%20Base%20Class%20References))
  (bind _maxnuminrow (Variables|Default|GetMaxNumInRow))
  (LocalVariables|SetlovWaveTotal WaveTotal)
  (LocalVariables|SetlocWaveEnemies WaveEnemies)
  (LocalVariables|SetWorldZvalue (.z (Variables|Default|GetSpawnLocationLeft)))
  (if (Variables|Default|GetbSpawnBoss)
    (CallFunction|SpawnWaveRtoL 0 (Variables|EnemyWave|GetBoss) (LocalVariables|GetWorldZvalue))
    (LocalVariables|SetWorldZvalue (- (LocalVariables|GetWorldZvalue) 8e+02))
    (Variables|Default|SetbSpawnBoss false))
  (if (< (/ (LocalVariables|GetlovWaveTotal) (Variables|Default|GetMaxNumInRow)) 1)
    ;[1 1 1] If num of Enemies is less then MaxNumInRow
    (CallFunction|SpawnWaveLtoR (LocalVariables|GetlovWaveTotal) (LocalVariables|GetlocWaveEnemies) (LocalVariables|GetWorldZvalue))
    (else
      (for _index (range 1 (/ (LocalVariables|GetlovWaveTotal) (Variables|Default|GetMaxNumInRow)))
        (if (LocalVariables|GetWaveLtoR)
          ;[1 1 1] iterates between spawning LtoR and RtoL
          (CallFunction|SpawnWaveLtoR _maxnuminrow (LocalVariables|GetlocWaveEnemies) (LocalVariables|GetWorldZvalue))
          (else
            (CallFunction|SpawnWaveRtoL _maxnuminrow (LocalVariables|GetlocWaveEnemies) (LocalVariables|GetWorldZvalue))))
        (LocalVariables|SetWaveLtoR (not (LocalVariables|GetWaveLtoR)))
        (LocalVariables|SetWorldZvalue (- (LocalVariables|GetWorldZvalue) 5e+02)))
      (if (LocalVariables|GetWaveLtoR)
        ;[1 1 1] Spawns the remaining of the wave total
        (CallFunction|SpawnWaveLtoR (Math|Float|Truncate (* (Variables|Default|GetMaxNumInRow) (Math|Float|Fraction (/ (Math|Conversions|ToFloat(Integer) (LocalVariables|GetlovWaveTotal)) (Math|Conversions|ToFloat(Integer) (Variables|Default|GetMaxNumInRow)))))) (LocalVariables|GetlocWaveEnemies) (LocalVariables|GetWorldZvalue))
        (else
          (CallFunction|SpawnWaveRtoL (Math|Float|Truncate (* (Variables|Default|GetMaxNumInRow) (Math|Float|Fraction (/ (Math|Conversions|ToFloat(Integer) (LocalVariables|GetlovWaveTotal)) (Math|Conversions|ToFloat(Integer) (Variables|Default|GetMaxNumInRow)))))) (LocalVariables|GetlocWaveEnemies) (LocalVariables|GetWorldZvalue)))))))

(fn SpawnWaveLtoR
  (params (WaveTotal :type Integer) (WaveEnemies :type Array%20of%20BP%20Enemy%20Base%20Class%20References) (WorldZValue :type Float%20%28single-precision%29))
  (bind _spawnlocationleft (Variables|Default|GetSpawnLocationLeft))
  (for _index (range 1 WaveTotal)
    (Game|SpawnActorfromClass (Utilities|Array|Get(acopy) WaveEnemies (Math|Random|RandomInteger (Utilities|Array|Length WaveEnemies))) (Math|Transform|MakeTransform (Math|Vector|MakeVector (- (.x _spawnlocationleft) (* _index (Variables|Float|GetStep))) (.y _spawnlocationleft) WorldZValue) "0, 0, 0" "0.700000,0.700000,0.700000") "Undefined" 0 0)))

(fn SpawnWaveRtoL
  (params (WaveTotal :type Integer) (WaveEnemies :type Array%20of%20BP%20Enemy%20Base%20Class%20References) (WorldZValue :type Float%20%28single-precision%29))
  (bind _spawnlocationright (Variables|Default|GetSpawnLocationRight))
  (for _index (range 0 WaveTotal)
    (bind _returnvalue (Game|SpawnActorfromClass (Utilities|Array|Get(acopy) WaveEnemies (Math|Random|RandomInteger (Utilities|Array|Length WaveEnemies))) (Math|Transform|MakeTransform (Math|Vector|MakeVector (+ (* _index (Variables|Float|GetStep)) (.x _spawnlocationright)) (.y _spawnlocationright) WorldZValue) "0, 0, 0" "0.700000,0.700000,0.700000") "Undefined" 0 0))
    (Variables|/Game/Blueprints/Enemies/BPEnemyBase.BPEnemyBase_C|SetbMoveRight _returnvalue false)))