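; BPEnemyThree is an enemy Blueprint that fires a laser in timed bursts, extending parent Tick logic.
; Tick alternates a LaserOn flag through Delays: off for FireRate, then on for 1.3 seconds with a shot sound.
; While on, it spawns a BPLaserEnemy at ProjectileSpawn every frame, forming a continuous stream.
; The construction script sets a fixed rotation on EnemyMesh.
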(event EventBeginPlay
  (|CallParentFunction) ; This node is disabled and will not be called.\nDrag off pins to build functionality.
)

(event Collision|EventActorBeginOverlap
  (params (OtherActor :type Actor%20Object%20Reference)))

(event EventTick
  (params (DeltaSeconds :type Float%20%28single-precision%29))
  (|CallParentFunction DeltaSeconds)
  (if (Variables|Default|GetLaserOn)
    (Game|SpawnActorfromClass "/Game/Blueprints/Projectiles/BPLaserEnemy.BPLaserEnemy_C" (Math|Transform|MakeTransform (Transformation|GetWorldLocation (Variables|Default|GetProjectileSpawn)) "0, 0, 0" "1,1,1") "Undefined" 0 0)
    (Utilities|FlowControl|Delay 1.3)
    (Variables|Default|SetLaserOn false)
    (else
      (Utilities|FlowControl|Delay (Variables|Default|GetFireRate))
      (Variables|Default|SetLaserOn true)
      (Audio|PlaySoundatLocation "/Game/Audio/SpaceLaserShot.SpaceLaserShot" "0, 0, 0" "0, 0, 0" 0.5 1.0 0.0 0 0 0))))

(fn ConstructionScript
  (|CallParentFunction)
  (Transformation|SetRelativeRotation (Variables|Default|GetEnemyMesh) "0.000000,90.000000,-90.000000" false false))