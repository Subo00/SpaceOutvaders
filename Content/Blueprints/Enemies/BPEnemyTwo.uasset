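; BPEnemyTwo is an enemy Blueprint that fires paired projectiles at randomized intervals.
; Tick calls the parent, then runs a Delay between FireRate and FireRate plus DropRate, which acts as a repeating fire timer because it ignores calls while pending.
; When the delay ends, it spawns a BPProjectileEnemyTwo at both the Left and Right component transforms and plays a quieter, higher-pitched EnemyShot sound at the actor.
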(event EventBeginPlay
  (|CallParentFunction) ; This node is disabled and will not be called.\nDrag off pins to build functionality.
)

(event Collision|EventActorBeginOverlap
  (params (OtherActor :type Actor%20Object%20Reference)))

(event EventTick
  (params (DeltaSeconds :type Float%20%28single-precision%29))
  (bind _firerate (Variables|Default|GetFireRate))
  (|CallParentFunction DeltaSeconds)
  (Utilities|FlowControl|Delay (Math|Random|RandomFloatinRange _firerate (+ _firerate (Variables|Default|GetDropRate))))
  (Game|SpawnActorfromClass "/Game/Blueprints/Projectiles/BPProjectileEnemyTwo.BPProjectileEnemyTwo_C" (Transformation|GetWorldTransform (Variables|Default|GetLeft)) "Undefined" 0 0)
  (Game|SpawnActorfromClass "/Game/Blueprints/Projectiles/BPProjectileEnemyTwo.BPProjectileEnemyTwo_C" (Transformation|GetWorldTransform (Variables|Default|GetRight)) "Undefined" 0 0)
  (Audio|PlaySoundatLocation "/Game/Audio/EnemyShot.EnemyShot" (Transformation|GetActorLocation) "0, 0, 0" 0.3 1.5 0.0 0 0 0))

(fn ConstructionScript
  (|CallParentFunction))