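; Health pickup actor that restores the player's health when its mesh is overlapped.
; On overlap with a BPPlayer it adds AddHP to CurrentHealth.
; Any amount above MaxHealth is truncated to an integer and awarded as score through BPGameMode, with health capped at the maximum.
; The pickup then destroys itself.
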(event OnComponentBeginOverlap(PickUpMesh)
  (params (OverlappedComponent :type Primitive%20Component%20Object%20Reference) (OtherActor :type Actor%20Object%20Reference) (OtherComp :type Primitive%20Component%20Object%20Reference) (OtherBodyIndex :type Integer) (bFromSweep :type Boolean) (SweepResult :type Hit%20Result%20Structure%20%28by%20ref%29))
  (bind _asbpplayer (Utilities|Casting|CastToBPPlayer OtherActor))
  (bind _output_get (Variables|/Game/Blueprints/Misc/BPPlayer.BPPlayer_C|SetCurrentHealth _asbpplayer (+ (Variables|/Game/Blueprints/Misc/BPPlayer.BPPlayer_C|GetCurrentHealth _asbpplayer) (Variables|Default|GetaddHP))))
  (if (> _output_get (Variables|/Game/Blueprints/Misc/BPPlayer.BPPlayer_C|GetMaxHealth _asbpplayer))
    ;[1 1 1] Adds excess health to score
    (bind _asbpgame_mode (Utilities|Casting|CastToBPGameMode (Game|GetGameMode)))
    (Default|AddScore _asbpgame_mode (Math|Float|Truncate (- _output_get (Variables|/Game/Blueprints/Misc/BPPlayer.BPPlayer_C|GetMaxHealth _asbpplayer))))
    (Variables|/Game/Blueprints/Misc/BPPlayer.BPPlayer_C|SetCurrentHealth _asbpplayer (Variables|/Game/Blueprints/Misc/BPPlayer.BPPlayer_C|GetMaxHealth _asbpplayer)))
  (Actor|DestroyActor))

(event EventBeginPlay)

(event Collision|EventActorBeginOverlap
  (params (OtherActor :type Actor%20Object%20Reference)))

(event EventTick
  (params (DeltaSeconds :type Float%20%28single-precision%29))
  (|CallParentFunction DeltaSeconds) ; This node is disabled and will not be called.\nDrag off pins to build functionality.
)

(fn ConstructionScript
  (|CallParentFunction))