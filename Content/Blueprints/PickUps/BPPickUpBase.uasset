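; Base pickup Blueprint that drifts along the Z axis at a default speed until it homes in on the player.
; A Box overlap stores the first BPPlayer that enters as the homing target.
; Each Tick eases the ProjectileMovement velocity toward that player at an increased speed using a fixed-alpha lerp, reverting to the default drift if no valid player is stored.
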(event OnComponentBeginOverlap(Box)
  (params (OverlappedComponent :type Primitive%20Component%20Object%20Reference) (OtherActor :type Actor%20Object%20Reference) (OtherComp :type Primitive%20Component%20Object%20Reference) (OtherBodyIndex :type Integer) (bFromSweep :type Boolean) (SweepResult :type Hit%20Result%20Structure%20%28by%20ref%29))
  ;[1 1 1] Homing Radious Control
  (bind _asbpplayer (Utilities|Casting|CastToBPPlayer OtherActor))
  (Utilities|IsValid (Variables|Default|GetBPPlayer)
    (:Is%20Not%20Valid
      (Variables|Default|SetBPPlayer _asbpplayer))))

(event EventTick
  (params (DeltaSeconds :type Float%20%28single-precision%29))
  (bind _projectilemovement (Variables|Default|GetProjectileMovement))
  ;[1 1 1] Movement Control
  (Utilities|IsValid (Variables|Default|GetBPPlayer)
    (:Is%20Valid
      (Variables|/Script/Engine.MovementComponent|SetVelocity (Variables|Default|GetProjectileMovement) (Math|Vector|Lerp(Vector) (Variables|/Script/Engine.MovementComponent|GetVelocity _projectilemovement) (* (Math|Vector|Normalize (- (Transformation|GetActorLocation (Variables|Default|GetBPPlayer)) (Transformation|GetActorLocation))) (Variables|Default|GetIncreasedSpeed)) 0.1)))
    (:Is%20Not%20Valid
      (Variables|/Script/Engine.MovementComponent|SetVelocity _projectilemovement (Math|Vector|MakeVector 0.0 0.0 (Variables|Default|GetDefaultSpeed))))))

(fn ConstructionScript)