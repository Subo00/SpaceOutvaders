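; Player actor for a shooter that slides along X, fires projectiles and creates its HUD outside the main menu.
; Tick eases horizontal speed toward input with FInterpTo, moves with sweep, and runs a Gate-held, cooldown-limited fire loop.
; Pickups start or extend a timed power-up, counted down by a recursive one-second delay, that swaps single shots for a pitch-spread volley.
; Damage reduces health; death flags BPGameMode, shows Game Over and destroys the actor.
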(event Custom|MoveRight
  ;[1 1 1] Use this for mobile input
  (bind _return_direction (CallFunction|GetDirection (Variables|Float|GetHozSpeed) 1e+01))
  (Variables|Float|SetHozSpeed _return_direction))

(event Custom|MoveLeft
  ;[1 1 1] Use this for mobile input
  (bind _return_direction (CallFunction|GetDirection (Variables|Float|GetHozSpeed) -1e+01))
  (Variables|Float|SetHozSpeed _return_direction))

(event Custom|FireRateControl
  (bind _projectilespawn (Variables|Default|GetProjectileSpawn))
  ;[1 1 1] Shooting
  (bind _output_get (Variables|Float|SetPrimaryFireRate (- (Variables|Float|GetPrimaryFireRate) (Variables|Float|GetDeltaSeconds))))
  (if (<= _output_get 0.0)
    (Utilities|FlowControl|Gate true
      (:Exit
        (Variables|Float|SetPrimaryFireRate (Variables|Float|GetPrimaryFireRateBase))
        (if (Variables|Default|GetbHasPower)
          (CallFunction|PowerUpFire (Variables|Integer|GetPowerShotCount) _projectilespawn)
          (else
            (CallFunction|PrimaryFire _projectilespawn)))
        (Audio|PlaySoundatLocation "/Game/Audio/Shot.Shot" (Transformation|GetActorLocation) "0, 0, 0" 0.3 1.0 0.0 0 0 0)))))

(event Custom|PowerUpDuration
  ;[1 1 1] PowerUpDuration
  (Utilities|FlowControl|Delay 1.0)
  (bind _output_get (Variables|Integer|SetPowerTime (- (Variables|Integer|GetPowerTime) 1)))
  (if (<= _output_get 0)
    (Variables|Default|SetbHasPower false)
    (Widget|SetVisibility (Variables|/Game/Blueprints/UI/HUD.HUD_C|GetPowerUpBox (Variables|Default|GetHUDReference)) "Hidden")
    (else
      (CallFunction|PowerUpDuration))))

(event EventBeginPlay
  ;[1 1 1] BeginPlay
  (bind _returnvalue (Game|GetCurrentLevelName true))
  (if (Utilities|Enum|NotEqual(Enum) _returnvalue "MainMenuMap")
    (Variables|Float|SetCurrentHealth (Variables|Float|GetMaxHealth))
    (bind _returnvalue_2 (UserInterface|CreateWidget "/Game/Blueprints/UI/HUD.HUD_C"))
    (bind _output_get (Variables|Default|SetHUDReference _returnvalue_2))
    (UserInterface|Viewport|AddtoViewport _output_get 0)))

(event Collision|EventActorBeginOverlap
  (params (OtherActor :type Actor%20Object%20Reference)))

(event EventTick
  (params (DeltaSeconds :type Float%20%28single-precision%29))
  ;[1 1 1] Old movement
  (Variables|Float|SetDeltaSeconds DeltaSeconds)
  (CallFunction|FireRateControl)
  (Utilities|FlowControl|Sequence
    (:then_0
      (bind _return_direction (CallFunction|GetDirection (Variables|Float|GetHozSpeed) (Input|AxisValues|GetMoveRight)))
      (Variables|Float|SetHozSpeed _return_direction))
    (:then_1
      (Transformation|SetActorLocation (+ (Transformation|GetActorLocation) (Math|Vector|MakeVector (Variables|Float|GetHozSpeed) 0.0 0.0)) true false))))

(event Game|Damage|EventAnyDamage
  (params (Damage :type Float%20%28single-precision%29) (DamageType :type Damage%20Type%20Object%20Reference) (InstigatedBy :type Controller%20Object%20Reference) (DamageCauser :type Actor%20Object%20Reference))
  ;[1 1 1] Player Death
  (Variables|Float|SetCurrentHealth (Math|Float|Clamp(Float) (- (Variables|Float|GetCurrentHealth) Damage) 0.0 (Variables|Float|GetMaxHealth)))
  (if (<= (Variables|Float|GetCurrentHealth) 0.0)
    (bind _asbpgame_mode (Utilities|Casting|CastToBPGameMode (Game|GetGameMode)))
    (Variables|/Game/Blueprints/Misc/BPGameMode.BPGameMode_C|SetbPlayerDead _asbpgame_mode true)
    (Default|PlaceWidget _asbpgame_mode "/Game/Blueprints/UI/GameOverMenu.GameOverMenu_C")
    (Actor|DestroyActor)))

(event Input|ActionEvents|InputActionPrimaryFire
  (params (Key :type Key%20Structure :default "None"))
  (bind _projectilespawn (Variables|Default|GetProjectileSpawn))
  ;[1 1 1] Shooting
  (:Pressed
    (Utilities|FlowControl|Gate true) ; enters at Open
  )
  (:Released
    (Utilities|FlowControl|Gate true) ; enters at Close
  ))

(fn ConstructionScript)

(fn GetDirection
  (params (Speed :type Float%20%28single-precision%29) (Direction :type Float%20%28single-precision%29))
  (bind _deltaseconds (Variables|Float|GetDeltaSeconds))
  (bind _output_get (Variables|Float|SetCurrentSpeed (Math|Interpolation|FInterpTo Speed (* (* Direction (Variables|Float|GetMovementSpeed)) _deltaseconds) _deltaseconds 4.0)))
  (return _output_get))

(fn PrimaryFire
  (params (SpawnLocation :type Scene%20Component%20Object%20Reference))
  (Game|SpawnActorfromClass "/Game/Blueprints/Projectiles/BPProjectilePlayerPrimary.BPProjectilePlayerPrimary_C" (Transformation|GetWorldTransform SpawnLocation) "AlwaysSpawn" 0 0))

(fn PowerUpPick
  (if (Variables|Default|GetbHasPower)
    (Variables|Integer|SetPowerTime (+ (Variables|Integer|GetPowerTime) (Variables|Integer|GetaddPowerTime)))
    (else
      (Variables|Default|SetbHasPower true)
      (Widget|SetVisibility (Variables|/Game/Blueprints/UI/HUD.HUD_C|GetPowerUpBox (Variables|Default|GetHUDReference)) "Visible")
      (Variables|Integer|SetPowerTime (Variables|Integer|GetaddPowerTime))
      (CallFunction|PowerUpDuration))))

(fn PowerUpFire
  (params (NumOfShots :type Integer) (SpawnLocation :type Scene%20Component%20Object%20Reference))
  (bind _returnvalue (Transformation|GetWorldTransform SpawnLocation))
  (bind (_location _rotation) (Math|Transform|BreakTransform _returnvalue))
  (LocalVariables|SetOffset (/ NumOfShots -2))
  (for _index (range 0 NumOfShots)
    (Game|SpawnActorfromClass "/Game/Blueprints/Projectiles/BPProjectilePlayerPowerd.BPProjectilePlayerPowerd_C" (Math|Transform|MakeTransform _location (Math|Rotator|MakeRotator 0.0 (+ (.pitch _rotation) (* (Math|Conversions|ToFloat(Integer) (LocalVariables|GetOffset)) 5.0)) 0.0)) "Undefined" 0 0)
    (LocalVariables|SetOffset (+ (LocalVariables|GetOffset) 1))))