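; BPGameMode is a game mode Blueprint that tracks the score and live enemy count and offers shared camera shake and menu helpers.
; BeginPlay caches the player pawn as BPPlayer, while AddEnemy, RemoveEnemy and AddScore update the counters.
; CallCamShake plays a world camera shake with an outer radius limit.
; PlaceWidget creates and displays a given widget, shows the mouse cursor and switches input to Game and UI, focused on that widget.
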(event Custom|CallCamShake
  (Camera|PlayWorldCameraShake "/Script/Engine.CameraShake" "0, 0, 0" -1.0 5e+02))

(event Custom|Place%20Widget
  (params (WidgetClass :type User%20Widget%20Class%20Reference))
  (bind _returnvalue (Game|GetPlayerController 0))
  (bind _returnvalue_2 (UserInterface|CreateWidget WidgetClass))
  (bind _output_get (Variables|Default|SetGameMenuReference _returnvalue_2))
  (UserInterface|Viewport|AddtoViewport _output_get 0)
  (Variables|/Script/Engine.PlayerController|SetbShowMouseCursor _returnvalue true)
  (Input|SetInputModeGameandUI _returnvalue _returnvalue_2 "DoNotLock" true))

(event EventBeginPlay
  (bind _asbpplayer (Utilities|Casting|CastToBPPlayer (Game|Player|GetPlayerPawn 0)))
  (Variables|Default|SetBPPlayer _asbpplayer))

(fn ConstructionScript)

(fn AddEnemy
  (Variables|Integer|SetLiveEnemies (+ (Variables|Integer|GetLiveEnemies) 1)))

(fn RemoveEnemy
  (Variables|Integer|SetLiveEnemies (- (Variables|Integer|GetLiveEnemies) 1)))

(fn AddScore
  (params (Score%20to%20Add :type Integer))
  (Variables|Integer|SetScore (+ Score%20to%20Add (Variables|Integer|GetScore))))