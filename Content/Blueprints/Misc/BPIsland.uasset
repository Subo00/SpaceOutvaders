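; BPIsland is an island Blueprint that places randomly chosen trees on itself.
; The Construction Script collects the relative transforms of five Arrow components into a SpawnPoints array, using them as placement markers.
; It then adds a static mesh component at each point with a random mesh from the Trees array, so the selection re-rolls whenever construction reruns.
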(fn ConstructionScript
  (CallFunction|SetSpawnPonts)
  (CallFunction|SpawnTrees))

(fn SetSpawnPonts
  (Variables|Default|SetSpawnPoints (Utilities|Array|MakeArray (Transformation|GetRelativeTransform (Variables|Default|GetArrow)) (Transformation|GetRelativeTransform (Variables|Default|GetArrow1)) (Transformation|GetRelativeTransform (Variables|Default|GetArrow2)) (Transformation|GetRelativeTransform (Variables|Default|GetArrow3)) (Transformation|GetRelativeTransform (Variables|Default|GetArrow4)))))

(fn SpawnTrees
  (bind _spawnpoints (Variables|Default|GetSpawnPoints))
  (bind _trees (Variables|Default|GetTrees))
  ;[1 1 1] Prođe kroz točke odnonsno Arrows
  (for _index (range 0 (- (Utilities|Array|Length _spawnpoints) 1))
    (bind _returnvalue (AddComponent|AddStaticMeshComponent false (Utilities|Array|Get(acopy) _spawnpoints _index)))
    ;[1 1 1] nadoda im stabla na random
    (Components|StaticMesh|SetStaticMesh _returnvalue (Utilities|Array|Get(acopy) _trees (Math|Random|RandomIntegerinRange 0 (Utilities|Array|LastIndex _trees))))))